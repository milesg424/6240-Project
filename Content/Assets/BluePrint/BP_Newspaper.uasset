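; BP_Newspaper is an interactable newspaper actor that opens an editing UI when the first-person character uses it.
; Entering its Box shows a TextRender and binds EditNewsPaper to the character's OnUseItem, unless Submit is already set.
; Using it switches to UI-only input with a cursor and adds two BP_UI widgets to the viewport.
; It then shares the end-overlap path, which hides the text and unbinds via that event's OtherActor.
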(event OnComponentBeginOverlap(Box)
  (params (OverlappedComponent :type Primitive%20Component%20Object%20Reference) (OtherActor :type Actor%20Object%20Reference) (OtherComp :type Primitive%20Component%20Object%20Reference) (OtherBodyIndex :type Integer) (bFromSweep :type Boolean) (SweepResult :type Hit%20Result%20Structure%20%28by%20ref%29))
  (bind _asbp_first_person_character (Utilities|Casting|CastToBP_FirstPersonCharacter OtherActor))
  (if (not (Variables|/Game/FirstPerson/Blueprints/BP_FirstPersonCharacter.BP_FirstPersonCharacter_C|Getsubmit _asbp_first_person_character))
    (Development|SetHiddeninGame (Variables|Default|GetTextRender) false false)
    (EventDispatchers|BindEventtoOnUseItem _asbp_first_person_character (delegate Custom|Edit%20NewsPaper))))

(event OnComponentEndOverlap(Box)
  (params (OverlappedComponent :type Primitive%20Component%20Object%20Reference) (OtherActor :type Actor%20Object%20Reference) (OtherComp :type Primitive%20Component%20Object%20Reference) (OtherBodyIndex :type Integer))
  (Development|SetHiddeninGame (Variables|Default|GetTextRender) true false)
  (bind _asbp_first_person_character (Utilities|Casting|CastToBP_FirstPersonCharacter OtherActor))
  (EventDispatchers|UnbindEventfromOnUseItem _asbp_first_person_character (delegate Custom|Edit%20NewsPaper)))

(event Custom|Edit%20NewsPaper
  (bind _returnvalue (Game|GetPlayerController 0))
  (Input|SetInputModeUIOnly _returnvalue 0 "DoNotLock" false)
  (Variables|/Script/Engine.PlayerController|SetbShowMouseCursor _returnvalue true)
  (bind _returnvalue_2 (UserInterface|CreateWidget "/Game/Assets/BluePrint/BP_UI.BP_UI_C"))
  (UserInterface|Viewport|AddtoViewport _returnvalue_2 0)
  (bind _returnvalue_3 (UserInterface|CreateWidget "/Game/Assets/BluePrint/BP_UI.BP_UI_C"))
  (UserInterface|Viewport|AddtoViewport _returnvalue_3 0)
  (Development|SetHiddeninGame (Variables|Default|GetTextRender) true false)
  (bind _asbp_first_person_character (Utilities|Casting|CastToBP_FirstPersonCharacter (stale OnComponentEndOverlap(Box) OtherActor)))
  (EventDispatchers|UnbindEventfromOnUseItem _asbp_first_person_character (delegate Custom|Edit%20NewsPaper)))

(event EventBeginPlay)

(event Collision|EventActorBeginOverlap
  (params (OtherActor :type Actor%20Object%20Reference)))

(event EventTick
  (params (DeltaSeconds :type Float%20%28single-precision%29)))

(fn ConstructionScript)